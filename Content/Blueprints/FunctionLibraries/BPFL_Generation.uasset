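; Blueprint function library of helpers for procedural prop generation built around BP_GenerativeProp.
; GetBoundsForGenerativeActor uses a generative prop's own bounds, otherwise colliding-component bounds with the origin offset by ParentProp's location, and flags which case applied.
; InitializeGenerativeProp passes the random stream, parent, dirtiness, density and debug flag to a generative prop, then calls Generate.
; It returns true even when the cast fails.
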(fn `Get Bounds For Generative Actor`
  (params (Actor :type "Actor Object Reference") (`Parent Prop` :type "Actor Object Reference"))
  (returns (Origin :type "Vector Structure") (Extent :type "Vector Structure") (`Is Generative Prop` :type Boolean))
  (bind (_origin _boxextent) (`Actor.GetActorBounds` Actor true false))
  (bind _asbp_generative_prop (cast `/Game/Blueprints/BP_GenerativeProp` Actor)
    (:`then`
      (bind (_origin_2 _boxextent_2) (`/Game/Blueprints/BP_GenerativeProp.GetBounds` _asbp_generative_prop))
      (return _origin_2 _boxextent_2 true))
    (:`CastFailed`
      (return (+ (`Actor.K2_GetActorLocation` `Parent Prop`) _origin) _boxextent false))))

(fn `Initialize Generative Prop`
  (params (Actor :type "Actor Object Reference") (`Prop Parent Actor` :type "Actor Object Reference") (`Random Stream` :type "RandomStream Structure") (Dirtiness :type "Float (double-precision)") (`Prop Density` :type "Float (double-precision)") (`Show Debug Spawn Points` :type Boolean))
  (returns (`Cast Success` :type Boolean))
  (bind _asbp_generative_prop (cast `/Game/Blueprints/BP_GenerativeProp` Actor)
    (:`then`
      (set `/Game/Blueprints/BP_GenerativeProp.Random Stream` `Random Stream` _asbp_generative_prop)
      (set `/Game/Blueprints/BP_GenerativeProp.Prop Parent Actor` `Prop Parent Actor` _asbp_generative_prop)
      (set `/Game/Blueprints/BP_GenerativeProp.Dirtiness` Dirtiness _asbp_generative_prop)
      (set `/Game/Blueprints/BP_GenerativeProp.Prop Density` `Prop Density` _asbp_generative_prop)
      (set `/Game/Blueprints/BP_GenerativeProp.Show Debug Spawn Points` `Show Debug Spawn Points` _asbp_generative_prop)
      (`/Game/Blueprints/BP_GenerativeProp.Generate` _asbp_generative_prop)
      (return true))
    (:`CastFailed`
      (return true))))