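; Blueprint function library for deterministic random sampling, with a single function that returns a random point inside a rotated box.
; RandomPointInBoundingBox draws each axis offset from the supplied random stream within plus or minus the extent, rotates it, then adds the location.
; Using a random stream instead of global random makes results repeatable for a given seed.
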(fn `RandomPointInBoundingBox`
  (params (`Random Stream` :type "RandomStream Structure") (Location :type "Vector Structure") (Extent :type "Vector Structure") (Rotation :type "Rotator Structure"))
  (returns (Point :type "Vector Structure"))
  (bind _x (.x Extent))
  (bind _y (.y Extent))
  (bind _z (.z Extent))
  (return (+ (`KismetMathLibrary.GreaterGreater_VectorRotator` (`KismetMathLibrary.MakeVector` (`KismetMathLibrary.RandomFloatInRangeFromStream` (- 0.0 _x) _x `Random Stream`) (`KismetMathLibrary.RandomFloatInRangeFromStream` (- 0.0 _y) _y `Random Stream`) (`KismetMathLibrary.RandomFloatInRangeFromStream` (- 0.0 _z) _z `Random Stream`)) Rotation) Location)))