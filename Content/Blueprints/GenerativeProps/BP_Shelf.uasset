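; BP_Shelf is a procedural prop that builds a modular shelf from instanced static meshes.
; Generate clears all instances, picks maximum or seeded-random width and height, then places feet, shelf levels with end caps, and corner struts.
; Each instance receives Dirtiness as custom data, with optional debug spawn points.
; GetBounds returns a yaw-aware bounding box; BeginPlay and the construction script do not trigger generation.
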(fn `Generate`
  (locals (`Instance Height` :type Integer) (`Instance Row` :type Integer))
  (`|ExecutionSequence`
    (:`then_0`
      (`self.Remove`))
    (:`then_1`
      ;[1 1 1] Set dimensions
      (if (`self.Set To Max Dimensions`)
        (set `self.Width` (`self.Max Width`))
        (set `self.Height` (`self.Max Height`))
        (else
          (set `self.Width` (`KismetMathLibrary.RandomIntegerInRangeFromStream` 1 (`self.Max Width`) (`self.Random Stream`)))
          (set `self.Height` (`KismetMathLibrary.RandomIntegerInRangeFromStream` 1 (`self.Max Height`) (`self.Random Stream`))))))
    (:`then_2`
      ;[1 1 1] Genereate Feet
      (`|ExecutionSequence`
        (:`then_0`
          (`self.Add Instance At Location` (`KismetMathLibrary.MakeVector` -25.0 (* (`self.Width`) -25.0)) (struct :`R` 1.0 :`G` 0.854902 :`A` 1.0) (struct :`Yaw` 90.0) (`self.Shelf Feet`)))
        (:`then_1`
          (`self.Add Instance At Location` (`KismetMathLibrary.MakeVector` -25.0 (* (`self.Width`) 25.0)) (struct :`R` 1.0 :`G` 0.854902 :`A` 1.0) (struct) (`self.Shelf Feet`)))
        (:`then_2`
          (`self.Add Instance At Location` (`KismetMathLibrary.MakeVector` 25.0 (* (`self.Width`) 25.0)) (struct :`R` 1.0 :`G` 0.854902 :`A` 1.0) (struct :`Yaw` 270.0) (`self.Shelf Feet`)))
        (:`then_3`
          (`self.Add Instance At Location` (`KismetMathLibrary.MakeVector` 25.0 (* (`self.Width`) -25.0)) (struct :`R` 1.0 :`G` 0.854902 :`A` 1.0) (struct :`Yaw` 180.0) (`self.Shelf Feet`)))))
    (:`then_3`
      (for _index (range (+ (`self.Height`) 1))
        (set `local.Instance Height` _index)
        (`|ExecutionSequence`
          (:`then_0`
            ;[1 1 1] Generate middle shelf part
            (for _index_2 (range 2 (+ (`self.Width`) 1))
              (set `local.Instance Row` (- _index_2 1))
              (`self.Add Instance At Location` (`KismetMathLibrary.MakeVector` 0.0 (+ (* (`KismetMathLibrary.Conv_IntToDouble` (- (`local.Instance Row`) 1)) 50.0) (* (`KismetMathLibrary.Conv_IntToDouble` (- (`self.Width`) 2)) -25.0)) (+ (* (`KismetMathLibrary.Conv_IntToDouble` (`local.Instance Height`)) 50.0) 10.0)) (struct :`R` 1.0 :`G` 0.854902 :`A` 1.0) (struct) (`self.Shelf Levels Middle`))))
          (:`then_1`
            ;[1 1 1] Generate Shelf End Parts
            (`|ExecutionSequence`
              (:`then_0`
                (`self.Add Instance At Location` (`KismetMathLibrary.MakeVector` 0.0 (* (`KismetMathLibrary.Conv_IntToDouble` (- (`self.Width`) 1)) 25.0) (+ (* (`KismetMathLibrary.Conv_IntToDouble` (`local.Instance Height`)) 50.0) 10.0)) (struct :`R` 1.0 :`G` 0.854902 :`A` 1.0) (struct) (`self.Shelf Levels End Left`)))
              (:`then_1`
                (`self.Add Instance At Location` (`KismetMathLibrary.MakeVector` 0.0 (* (`KismetMathLibrary.Conv_IntToDouble` (- (`self.Width`) 1)) -25.0) (+ (* (`KismetMathLibrary.Conv_IntToDouble` (`local.Instance Height`)) 50.0) 10.0)) (struct :`R` 1.0 :`G` 0.854902 :`A` 1.0) (struct) (`self.Shelf Levels End Right`)))))
          (:`then_2`
            ;[1 1 1] Genereate Struts
            (if (< (`local.Instance Height`) (`self.Height`))
              (`|ExecutionSequence`
                (:`then_0`
                  (`self.Add Instance At Location` (`KismetMathLibrary.MakeVector` -25.0 (* (`self.Width`) -25.0) (+ (* (`KismetMathLibrary.Conv_IntToDouble` (`local.Instance Height`)) 50.0) 10.0)) (struct :`R` 1.0 :`G` 0.854902 :`A` 1.0) (struct :`Yaw` 90.0) (`self.Shelf Struts`)))
                (:`then_1`
                  (`self.Add Instance At Location` (`KismetMathLibrary.MakeVector` -25.0 (* (`self.Width`) 25.0) (+ (* (`KismetMathLibrary.Conv_IntToDouble` (`local.Instance Height`)) 50.0) 10.0)) (struct :`R` 1.0 :`G` 0.854902 :`A` 1.0) (struct) (`self.Shelf Struts`)))
                (:`then_2`
                  (`self.Add Instance At Location` (`KismetMathLibrary.MakeVector` 25.0 (* (`self.Width`) 25.0) (+ (* (`KismetMathLibrary.Conv_IntToDouble` (`local.Instance Height`)) 50.0) 10.0)) (struct :`R` 1.0 :`G` 0.854902 :`A` 1.0) (struct :`Yaw` 270.0) (`self.Shelf Struts`)))
                (:`then_3`
                  (`self.Add Instance At Location` (`KismetMathLibrary.MakeVector` 25.0 (* (`self.Width`) -25.0) (+ (* (`KismetMathLibrary.Conv_IntToDouble` (`local.Instance Height`)) 50.0) 10.0)) (struct :`R` 1.0 :`G` 0.854902 :`A` 1.0) (struct :`Yaw` 180.0) (`self.Shelf Struts`)))))))))))

(fn `GetBounds`
  (returns (Origin :type "Vector Structure") (BoxExtent :type "Vector Structure"))
  (bind _yaw (.yaw (`self.K2_GetActorRotation`)))
  (bind _returnvalue (* (`KismetMathLibrary.Conv_IntToDouble` (`self.Width`)) 0.25))
  (bind _returnvalue_2 (* _returnvalue -1.0))
  (bind (_x _y) (`KismetMathLibrary.BreakVector2D` (`KismetMathLibrary.GetRotated2D` (`KismetMathLibrary.MakeVector2D` _returnvalue 0.25) _yaw)))
  (bind (_x_2 _y_2) (`KismetMathLibrary.BreakVector2D` (`KismetMathLibrary.GetRotated2D` (`KismetMathLibrary.MakeVector2D` _returnvalue -0.25) _yaw)))
  (bind (_x_3 _y_3) (`KismetMathLibrary.BreakVector2D` (`KismetMathLibrary.GetRotated2D` (`KismetMathLibrary.MakeVector2D` _returnvalue_2 -0.25) _yaw)))
  (bind (_x_4 _y_4) (`KismetMathLibrary.BreakVector2D` (`KismetMathLibrary.GetRotated2D` (`KismetMathLibrary.MakeVector2D` _returnvalue_2 0.25) _yaw)))
  (bind _returnvalue_3 (`/Game/Blueprints/FunctionLibraries/BPFL_Vectors.Make Centimeter Vector From Meters` 0.0 0.0 (+ (* (`KismetMathLibrary.Conv_IntToDouble` (`self.Height`)) 0.25) 0.05)))
  (bind _returnvalue_4 (`/Game/Blueprints/FunctionLibraries/BPFL_Vectors.Make Centimeter Vector From Meters` (`KismetMathLibrary.FMax` _y _y_2 _y_4 _y_3) (`KismetMathLibrary.FMax` _x _x_2 _x_4 _x_3) (/ (+ (* (`KismetMathLibrary.Conv_IntToDouble` (`self.Height`)) 0.5) 0.1) 2.0)))
  (return (+ (`self.K2_GetActorLocation`) _returnvalue_3) _returnvalue_4))

(fn `Remove`
  (for _array_element (`self.K2_GetComponentsByClass` "/Script/Engine.InstancedStaticMeshComponent")
    (bind _asinstanced_static_mesh_component (cast `InstancedStaticMeshComponent` _array_element))
    (`InstancedStaticMeshComponent.ClearInstances` _asinstanced_static_mesh_component)))

(fn `UserConstructionScript`)