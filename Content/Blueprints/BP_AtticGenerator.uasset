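; BP_AtticGenerator procedurally builds a gabled attic sized by Length and Height on a one-metre grid.
; The construction script optionally runs GenerateAttic, placing instanced meshes for floor, sloped sides, rafters, end walls and struts, with optional debug points.
; It also adds hanging lights with point lights and scales dust particles to the attic volume.
; Tarps, end rafters, focal assets and BeginPlay prop generation are empty stubs.
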(event `self.ReceiveBeginPlay`
  (`|ExecutionSequence`
    (:`then_0`
      (if (`self.Generate Props On Play`)
        (`self.Clear Environment Meshes (TODO)`)
        (`self.Generate Environmental Meshes (TODO)`)))))

(fn `Clear Environment Meshes (TODO)`
  (for _array_element (`self.Spawned Actors`)
    (`self.K2_DestroyActor` _array_element)))

(fn `Generate Attic`
  (`|ExecutionSequence`
    (:`then_0`
      (`KismetSystemLibrary.FlushPersistentDebugLines`))
    (:`then_1`
      (`self.Generate Floor`))
    (:`then_2`
      (`self.Generate Side Walls And Rafters`))
    (:`then_3`
      (`self.Generate Wall Tarps (T ODO)`))
    (:`then_4`
      (`self.Generate Front Wall (TOFINISH)`))
    (:`then_5`
      (`self.Generate Front Rafters (TODO)`))
    (:`then_6`
      (`self.Generate Back Wall (TOFINISH)`))
    (:`then_7`
      (`self.Generate Back Rafters (TODO)`))
    (:`then_8`
      (`self.Generate Support Struts`))
    (:`then_9`
      (`self.Generate Hanging Lights`))
    (:`then_10`
      (`self.Generate Dust Particles`))
    (:`then_11`
      (`self.Generate Focal Assets (TODO)`))))

(fn `Generate Back Rafters (TODO)`)

(fn `Generate Back Wall (TOFINISH)`
  (`|ExecutionSequence`
    (:`then_0`
      ;[1 1 1] Set Meshes
      (`StaticMeshComponent.SetStaticMesh` (`self.Back Square Panels`) (`self.FrontSquareMesh`))
      (`StaticMeshComponent.SetStaticMesh` (`self.Triangle Right Panels`) (`self.FrontEdgeRightMesh`))
      (`StaticMeshComponent.SetStaticMesh` (`self.Triangle Left Panels`) (`self.FrontEdgeLeftMesh`)))
    (:`then_1`
      (for _index (range (+ (- (`self.Height`) 2) 1))
        (bind _returnvalue (- (* (- (`self.Height`) _index) 2) 3))
        (for _index_2 (range (+ _returnvalue 1))
          ;[1 1 1] Set square panels
          (`self.Add Instance At Location` (`self.Make Centimetre Vector From Metres` (- (`KismetMathLibrary.Conv_IntToDouble` (`self.Length`)) 0.5) (- (`KismetMathLibrary.Conv_IntToDouble` (+ _index_2 (* (/ _returnvalue 2) -1))) 0.5) (`KismetMathLibrary.Conv_IntToDouble` _index)) (struct :`Yaw` 180.0) (`self.Back Square Panels`) (struct :`G` 1.0 :`A` 1.0)))))
    (:`then_2`
      (for _index_3 (range (`self.Height`))
        (bind _returnvalue_2 (`self.Make Centimetre Vector From Metres` (- (`KismetMathLibrary.Conv_IntToDouble` (`self.Length`)) 0.5) (- (`KismetMathLibrary.Conv_IntToDouble` (- (`self.Height`) _index_3)) 0.5) (`KismetMathLibrary.Conv_IntToDouble` _index_3)))
        ;[1 1 1] Set side panels
        (`self.Add Instance At Location` _returnvalue_2 (struct :`Yaw` 180.0) (`self.Triangle Right Panels`) (struct :`G` 1.0 :`A` 1.0))
        (`self.Add Instance At Location` (* _returnvalue_2 (1.0 -1.0 1.0)) (struct :`Yaw` 180.0) (`self.Triangle Left Panels`) (struct :`G` 1.0 :`A` 1.0))))))

(fn `Generate Dust Particles`
  (bind _height (`self.Height`))
  (bind _returnvalue (`KismetMathLibrary.Conv_IntToDouble` (`self.Length`)))
  (bind _returnvalue_2 (`KismetMathLibrary.Conv_IntToDouble` (`self.Height`)))
  (bind _returnvalue_3 (* _returnvalue_2 2.0))
  ;[1 1 1] Place and Scale particle system so it covers the whole attic area
  (`SceneComponent.K2_SetRelativeTransform` (`self.Dust_Particles`) (`KismetMathLibrary.MakeTransform` (- (`self.Make Centimetre Vector From Metres` (/ _returnvalue 2.0) 0.0 (/ _returnvalue_2 2.0)) (50.0 0.0 50.0)) (struct) (/ (`KismetMathLibrary.MakeVector` _returnvalue _returnvalue_3 _returnvalue_3) (4.0 4.0 2.0))) false false)
  ;[1 1 1] Scale the spawn rate with the attic area so the particle density is constant
  (`NiagaraComponent.SetVariableFloat` (`self.Dust_Particles`) "Spawn Rate" (* (`self.Dirtiness`) 0.1 _height _height (`self.Length`))))

(fn `Generate Environmental Meshes (TODO)`)

(fn `Generate Floor`
  (bind _returnvalue (- (* (`self.Height`) 2) 1))
  (`|ExecutionSequence`
    (:`then_0`
      ;[1 1 1] Set Meshes
      (`StaticMeshComponent.SetStaticMesh` (`self.Floor Square Panels`) (`self.FloorPanelMesh`)))
    (:`then_1`
      (for _index (range (+ _returnvalue 1))
        (for _index_2 (range (`self.Length`))
          (`self.Add Instance At Location` (`self.Make Centimetre Vector From Metres` (`KismetMathLibrary.Conv_IntToDouble` _index_2) (- (`KismetMathLibrary.Conv_IntToDouble` _index) (/ (`KismetMathLibrary.Conv_IntToDouble` _returnvalue) 2.0))) (struct) (`self.Floor Square Panels`) (struct :`G` 1.0 :`B` 1.0 :`A` 1.0)))))))

(fn `Generate Focal Assets (TODO)`)

(fn `Generate Front Rafters (TODO)`)

(fn `Generate Front Wall (TOFINISH)`
  (`|ExecutionSequence`
    (:`then_0`
      ;[1 1 1] Set Meshes
      (`StaticMeshComponent.SetStaticMesh` (`self.Front Square Panels`) (`self.FrontSquareMesh`))
      (`StaticMeshComponent.SetStaticMesh` (`self.Triangle Right Panels`) (`self.FrontEdgeRightMesh`))
      (`StaticMeshComponent.SetStaticMesh` (`self.Triangle Left Panels`) (`self.FrontEdgeLeftMesh`)))
    (:`then_1`
      ;[1 1 1] Set square meshes
      (for _index (range (+ (- (`self.Height`) 2) 1))
        (bind _returnvalue (- (* (- (`self.Height`) _index) 2) 3))
        (for _index_2 (range (+ _returnvalue 1))
          (`self.Add Instance At Location` (`self.Make Centimetre Vector From Metres` -0.5 (- (`KismetMathLibrary.Conv_IntToDouble` (+ _index_2 (* (/ _returnvalue 2) -1))) 0.5) (`KismetMathLibrary.Conv_IntToDouble` _index)) (struct) (`self.Front Square Panels`) (struct :`G` 1.0 :`A` 1.0)))))
    (:`then_2`
      ;[1 1 1] Set triangle meshes
      (for _index_3 (range (`self.Height`))
        (bind _returnvalue_2 (`self.Make Centimetre Vector From Metres` -0.5 (- (`KismetMathLibrary.Conv_IntToDouble` (- (`self.Height`) _index_3)) 0.5) (`KismetMathLibrary.Conv_IntToDouble` _index_3)))
        (`self.Add Instance At Location` _returnvalue_2 (struct) (`self.Triangle Left Panels`) (struct :`G` 1.0 :`A` 1.0))
        (`self.Add Instance At Location` (* _returnvalue_2 (1.0 -1.0 1.0)) (struct) (`self.Triangle Right Panels`) (struct :`G` 1.0 :`A` 1.0))))))

(fn `Generate Hanging Lights`
  (locals (`Wire Height` :type "Float (double-precision)") (`Wire Length` :type "Float (double-precision)") (`Current Point Light Component` :type "PointLightComponent Object Reference"))
  (`|ExecutionSequence`
    (:`then_0`
      ;[1 1 1] Set meshes
      (`StaticMeshComponent.SetStaticMesh` (`self.Wires`) (`self.HangingLightWireMesh`))
      (`StaticMeshComponent.SetStaticMesh` (`self.Shade`) (`self.HangingLightShadeMesh`)))
    (:`then_1`
      (for _index (range (+ (/ (- (`self.Length`) 4) 4) 1))
        (set `local.Wire Length` (+ (* (`KismetMathLibrary.Conv_IntToDouble` _index) 4.0) 2.5))
        (for _index_2 (range (`self.Point Light Height From Ground`) (`self.Height`))
          (set `local.Wire Height` (`KismetMathLibrary.Conv_IntToDouble` _index_2))
          ;[1 1 1] Place wires
          (`self.Add Instance At Location` (`self.Make Centimetre Vector From Metres` (`local.Wire Length`) 0.0 (`local.Wire Height`)) (struct) (`self.Wires`) (struct :`R` 1.0 :`B` 0.013448 :`A` 1.0)))
        (`|ExecutionSequence`
          (:`then_0`
            ;[1 1 1] Generate light shades
            (`self.Add Instance At Location` (`self.Make Centimetre Vector From Metres` (`local.Wire Length`) 0.0 (`KismetMathLibrary.Conv_IntToDouble` (`self.Point Light Height From Ground`))) (struct) (`self.Shade`) (struct :`A` 1.0)))
          (:`then_1`
            ;[1 1 1] Generate point lights
            (bind _returnvalue (`AddComponent|NODE_AddPointLightComponent-2` :`RelativeTransform` (`KismetMathLibrary.MakeTransform` (`self.Make Centimetre Vector From Metres` (`local.Wire Length`) 0.0 (`KismetMathLibrary.Conv_IntToDouble` (`self.Point Light Height From Ground`))))))
            (set `local.Current Point Light Component` _returnvalue)
            (`|ExecutionSequence`
              (:`then_0`
                (`LightComponent.SetIntensity` (`local.Current Point Light Component`) (`self.Point Light Intensity`)))
              (:`then_1`
                (`LocalLightComponent.SetAttenuationRadius` (`local.Current Point Light Component`) (* (+ (`KismetMathLibrary.Conv_IntToDouble` (`self.Height`)) (* (`KismetMathLibrary.Conv_IntToDouble` (`self.Point Light Height From Ground`)) 1.414214)) 100.0)))
              (:`then_2`
                (`LightComponent.SetTemperature` (`local.Current Point Light Component`) (`self.Point Light Temperature`))
                (`LightComponent.SetLightColor` (`local.Current Point Light Component`) (`self.Point Light Color`) true)))))))))

(fn `Generate Side Walls And Rafters`
  (locals (Column :type Integer) (Row :type Integer) (Location :type "Vector Structure"))
  (bind _returnvalue (`KismetMathLibrary.Conv_IntToDouble` (`local.Row`)))
  (bind _returnvalue_2 (`KismetMathLibrary.Conv_IntToDouble` (`local.Row`)))
  (`|ExecutionSequence`
    (:`then_0`
      ;[1 1 1] Set meshes
      (`StaticMeshComponent.SetStaticMesh` (`self.Side Square Panels`) (`self.SidePanelMesh`))
      (`StaticMeshComponent.SetStaticMesh` (`self.Side Vertical Rafters`) (`self.SideRafterVerticalMesh`))
      (`StaticMeshComponent.SetStaticMesh` (`self.Side Horizontal Rafters`) (`self.SideRafterHorizontalMesh`)))
    (:`then_1`
      (for _index (range (`self.Length`))
        (set `local.Column` _index)
        (for _index_2 (range (`self.Height`))
          (set `local.Row` _index_2)
          (set `local.Location` (`self.Make Centimetre Vector From Metres` (`KismetMathLibrary.Conv_IntToDouble` (`local.Column`)) (- (`KismetMathLibrary.Conv_IntToDouble` (`self.Height`)) _returnvalue_2) _returnvalue_2))
          (`|ExecutionSequence`
            (:`then_0`
              ;[1 1 1] Instance side panels
              (`self.Add Instance At Location` (`local.Location`) (struct :`Yaw` -90.0) (`self.Side Square Panels`) (struct :`G` 1.0 :`A` 1.0))
              (`self.Add Instance At Location` (* (`local.Location`) (1.0 -1.0 1.0)) (struct :`Yaw` 90.0) (`self.Side Square Panels`) (struct :`G` 1.0 :`A` 1.0)))
            (:`then_1`
              ;[1 1 1] Instance horizontal rafters
              (if (== (mod (`local.Row`) 2) 1)
                (`self.Add Instance At Location` (`local.Location`) (struct :`Yaw` -90.0) (`self.Side Horizontal Rafters`) (struct :`G` 1.0 :`A` 1.0))
                (`self.Add Instance At Location` (* (`local.Location`) (1.0 -1.0 1.0)) (struct :`Yaw` 90.0) (`self.Side Horizontal Rafters`) (struct :`G` 1.0 :`A` 1.0))))))))
    (:`then_2`
      (for _index_3 (range (+ (`self.Length`) 1))
        (set `local.Column` _index_3)
        (for _index_4 (range (`self.Height`))
          (set `local.Row` _index_4)
          (set `local.Location` (`self.Make Centimetre Vector From Metres` (`KismetMathLibrary.Conv_IntToDouble` (`local.Column`)) (- (`KismetMathLibrary.Conv_IntToDouble` (`self.Height`)) _returnvalue) _returnvalue))
          (`|ExecutionSequence`
            (:`then_0`
              ;[1 1 1] Instance vertical rafters
              (`self.Add Instance At Location` (- (`local.Location`) (50.0 0.0 0.0)) (struct :`Yaw` -90.0) (`self.Side Vertical Rafters`) (struct :`G` 1.0 :`A` 1.0)))
            (:`then_1`
              (`self.Add Instance At Location` (- (* (`local.Location`) (1.0 -1.0 1.0)) (50.0 0.0 0.0)) (struct :`Yaw` 90.0) (`self.Side Vertical Rafters`) (struct :`G` 1.0 :`A` 1.0)))))))))

(fn `Generate Support Struts`
  (bind _returnvalue (`self.Make Centimetre Vector From Metres` (- (`KismetMathLibrary.Conv_IntToDouble` (`self.Length`)) 0.5) (- (`KismetMathLibrary.Conv_IntToDouble` (`self.Height`)) 1.0)))
  (bind _returnvalue_2 (`self.Make Centimetre Vector From Metres` (- (`KismetMathLibrary.Conv_IntToDouble` (`self.Length`)) 0.5) (- (`KismetMathLibrary.Conv_IntToDouble` (`self.Height`)) 3.0)))
  (bind _returnvalue_3 (`self.Make Centimetre Vector From Metres` (- (`KismetMathLibrary.Conv_IntToDouble` (`self.Length`)) 0.5) 0.0 (- (`KismetMathLibrary.Conv_IntToDouble` (`self.Height`)) 2.0)))
  (`|ExecutionSequence`
    (:`then_0`
      ;[1 1 1] Set meshes
      (`StaticMeshComponent.SetStaticMesh` (`self.Top Vertical Struts`) (`self.TopStrutVerticalMesh`))
      (`StaticMeshComponent.SetStaticMesh` (`self.Top Horizontal Struts`) (`self.TopStrutHorizontalMesh`))
      (`StaticMeshComponent.SetStaticMesh` (`self.Side Vertical Strut 1m`) (`self.SideStrutVertical1mMesh`))
      (`StaticMeshComponent.SetStaticMesh` (`self.Side Vertical Strut 3m`) (`self.SideStrutVertical3mMesh`)))
    (:`then_1`
      ;[1 1 1] Generate Top Struts
      (for _index (range (+ (/ (`self.Length`) 2) 1))
        (bind _returnvalue_4 (`self.Make Centimetre Vector From Metres` (- (`KismetMathLibrary.Conv_IntToDouble` (* _index 2)) 0.5) 0.0 (- (`KismetMathLibrary.Conv_IntToDouble` (`self.Height`)) 2.0)))
        (`self.Add Instance At Location` _returnvalue_4 (struct :`Yaw` -90.0) (`self.Top Vertical Struts`) (struct :`G` 1.0 :`A` 1.0))
        (`self.Add Instance At Location` _returnvalue_4 (struct :`Yaw` -90.0) (`self.Top Horizontal Struts`) (struct :`G` 1.0 :`A` 1.0)))
      (`self.Add Instance At Location` _returnvalue_3 (struct :`Yaw` -90.0) (`self.Top Vertical Struts`) (struct :`G` 1.0 :`A` 1.0))
      (`self.Add Instance At Location` _returnvalue_3 (struct :`Yaw` -90.0) (`self.Top Horizontal Struts`) (struct :`G` 1.0 :`A` 1.0)))
    (:`then_2`
      ;[1 1 1] Generate small side struts
      (for _index_2 (range (+ (/ (- (`self.Length`) 1) 2) 1))
        (bind _returnvalue_5 (`self.Make Centimetre Vector From Metres` (- (`KismetMathLibrary.Conv_IntToDouble` (* _index_2 2)) 0.5) (- (`KismetMathLibrary.Conv_IntToDouble` (`self.Height`)) 1.0)))
        (`self.Add Instance At Location` _returnvalue_5 (struct :`Yaw` -90.0) (`self.Side Vertical Strut 1m`) (struct :`G` 1.0 :`A` 1.0))
        (`self.Add Instance At Location` (* _returnvalue_5 (1.0 -1.0 1.0)) (struct :`Yaw` 90.0) (`self.Side Vertical Strut 1m`) (struct :`G` 1.0 :`A` 1.0)))
      (`self.Add Instance At Location` _returnvalue (struct :`Yaw` -90.0) (`self.Side Vertical Strut 1m`) (struct :`G` 1.0 :`A` 1.0))
      (`self.Add Instance At Location` (* _returnvalue (1.0 -1.0 1.0)) (struct :`Yaw` 90.0) (`self.Side Vertical Strut 1m`) (struct :`G` 1.0 :`A` 1.0)))
    (:`then_3`
      ;[1 1 1] Generate tall side struts
      (for _index_3 (range (+ (/ (- (`self.Length`) 1) 4) 1))
        (bind _returnvalue_6 (`self.Make Centimetre Vector From Metres` (- (`KismetMathLibrary.Conv_IntToDouble` (* _index_3 4)) 0.5) (- (`KismetMathLibrary.Conv_IntToDouble` (`self.Height`)) 3.0)))
        (`self.Add Instance At Location` _returnvalue_6 (struct :`Yaw` -90.0) (`self.Side Vertical Strut 3m`) (struct :`G` 1.0 :`A` 1.0))
        (`self.Add Instance At Location` (* _returnvalue_6 (1.0 -1.0 1.0)) (struct :`Yaw` 90.0) (`self.Side Vertical Strut 3m`) (struct :`G` 1.0 :`A` 1.0)))
      (`self.Add Instance At Location` _returnvalue_2 (struct :`Yaw` -90.0) (`self.Side Vertical Strut 3m`) (struct :`G` 1.0 :`A` 1.0))
      (`self.Add Instance At Location` (* _returnvalue_2 (1.0 -1.0 1.0)) (struct :`Yaw` 90.0) (`self.Side Vertical Strut 3m`) (struct :`G` 1.0 :`A` 1.0)))))

(fn `Generate Wall Tarps (T ODO)`)

(fn `UserConstructionScript`
  (if (`self.Automatically Regenerate On Edit`)
    (`self.Generate Attic`)))