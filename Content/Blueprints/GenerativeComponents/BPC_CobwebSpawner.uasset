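; Generative component that scatters random cobweb props against world-static surfaces within a box on its parent prop actor.
; Generate spawns temporary probe props along each side and box-traces across the margin-reduced extent in four directions, using a seeded random stream.
; Hits spawn props by Dirtiness chance, culling overlaps within each sweep.
; Survivors are swept to the parent's height, tagged, attached to its Props socket and recorded in GeneratedActors.
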(fn `Generate`
  (locals (`Ray Origin` :type "Vector Structure") (`Ray Index` :type Integer) (`World Rotation` :type "Rotator Structure") (`Spawn Extent` :type "Vector Structure") (`Current Spawned Actor` :type "Actor Object Reference") (`Sweep Spawned Actor Set` :type "Set of Actor Object Reference") (`Sweep Actor` :type "Actor Object Reference") (`Sweep Actor Class` :type "Actor Class Reference") (`Sweep Hit Array` :type "Array of HitResult Structure") (`Draw Debug Type` :type "EDrawDebugTrace Enum" :default "None") (`Hit Actor` :type "Actor Object Reference"))
  (bind _margin (`self.Margin`))
  (bind _outitem (`KismetArrayLibrary.Array_RandomFromStream` (`self.Spawnable Props`) (`self.Random Stream`)))
  (bind _outitem_2 (`KismetArrayLibrary.Array_RandomFromStream` (`self.Spawnable Props`) (`self.Random Stream`)))
  (bind _outitem_3 (`KismetArrayLibrary.Array_RandomFromStream` (`self.Spawnable Props`) (`self.Random Stream`)))
  (bind _outitem_4 (`KismetArrayLibrary.Array_RandomFromStream` (`self.Spawnable Props`) (`self.Random Stream`)))
  (if (`self.Show Debug Spawn Points`)
    (`KismetSystemLibrary.DrawDebugBox` (+ (`self.Location`) (`Actor.K2_GetActorLocation` (`self.Prop Parent Actor`))) (`self.Extent`) (struct :`R` 0.17984 :`B` 0.401042 :`A` 1.0) (struct) 10.0 20.0))
  (if (`KismetArrayLibrary.Array_IsNotEmpty` (`self.Spawnable Props`))
    (`|ExecutionSequence`
      (:`then_0`
        (`KismetArrayLibrary.Array_Clear` (`self.Generated Actors`)))
      (:`then_1`
        ;[1 1 1] Adjust spawning extent and rotation
        (set `local.Spawn Extent` (- (`self.Extent`) (`KismetMathLibrary.MakeVector` _margin _margin _margin)))
        (bind _rotation (`/Game/Blueprints/FunctionLibraries/BPFL_Transform.Get Actor's World Rotation` (`self.Prop Parent Actor`)))
        (set `local.World Rotation` _rotation))
      (:`then_2`
        ;[1 1 1] Calculate X+ sweep locations
        (for _index (range (+ (`KismetMathLibrary.FTrunc` (* (.y (`local.Spawn Extent`)) 2.0 0.01)) 1))
          (set `local.Ray Index` _index)
          (`|ExecutionSequence`
            (:`then_0`
              (`BlueprintSetLibrary.Set_Clear` (`local.Sweep Spawned Actor Set`)))
            (:`then_1`
              ;;[1 1 1] Spawn actor for calculating sweeping
              (set `local.Sweep Actor Class` _outitem_2)
              (bind _returnvalue (`|SpawnActorFromClass` _outitem_2 (`KismetMathLibrary.MakeTransform` (+ (`KismetMathLibrary.GreaterGreater_VectorRotator` (+ (`KismetMathLibrary.MakeVector` 0.0 (+ (`KismetMathLibrary.RandomFloatInRangeFromStream` -25.0 25.0 (`self.Random Stream`)) (* (`local.Ray Index`) 100.0))) (* (-1.0 -1.0 0.0) (`local.Spawn Extent`))) (`local.World Rotation`)) (`self.Location`)) (`local.World Rotation`)) "AlwaysSpawn" "OverrideRootScale" null null))
              (set `local.Sweep Actor` _returnvalue))
            (:`then_2`
              ;;[1 1 1] Trace along sweep for hits
              (bind (_origin _extent) (`/Game/Blueprints/FunctionLibraries/BPFL_Generation.Get Bounds For Generative Actor` (`local.Sweep Actor`)))
              (bind _outhits (`KismetSystemLibrary.BoxTraceMultiForObjects` _origin (+ _origin (`KismetMathLibrary.GreaterGreater_VectorRotator` (+ (* (`local.Spawn Extent`) (2.0 0.0 0.0)) (100.0 0.0 0.0)) (`local.World Rotation`))) (- _extent (2.0 2.0 2.0)) (struct) (`|MakeArray` "ObjectTypeQuery1" :!type "EObjectTypeQuery Enum") false (`|MakeArray` (`local.Sweep Actor`)) (`local.Draw Debug Type`)))
              (set `local.Sweep Hit Array` _outhits)
              ;[1 1 1] Remove Hits in the same sweep if they collide
              (for _array_element (`local.Sweep Hit Array`) :!label _label
                (if (< (`KismetMathLibrary.RandomFloatInRangeFromStream` 0.0 5.0 (`self.Random Stream`)) (`self.Dirtiness`))
                  (bind _rotation_2 (`/Game/Blueprints/FunctionLibraries/BPFL_Transform.Get Actor's World Rotation` (`local.Sweep Actor`)))
                  (bind (_bblockinghit _binitialoverlap _time _distance _location _impactpoint _normal _impactnormal _physmat _hitactor) (`GameplayStatics.BreakHitResult` _array_element))
                  (bind _returnvalue_2 (`|SpawnActorFromClass` (`local.Sweep Actor Class`) (`KismetMathLibrary.MakeTransform` _location _rotation_2) "AlwaysSpawn" "OverrideRootScale" null null))
                  (bind _output_get (set `local.Current Spawned Actor` _returnvalue_2))
                  (bind _is_actor_colliding (`self.Is Actor Colliding with Set` _output_get (`local.Sweep Spawned Actor Set`)))
                  (if _is_actor_colliding
                    (`Actor.K2_DestroyActor` (`local.Current Spawned Actor`))
                    (else
                      (set `local.Hit Actor` _hitactor)
                      (if (`self.Show Debug Spawn Points`)
                        (`KismetSystemLibrary.DrawDebugArrow` _impactpoint (+ _impactpoint (* _impactnormal (100.0 100.0 100.0))) 4.0 (struct :`R` 0.047337 :`G` 1.0 :`A` 1.0) 10.0 1.0))
                      (`|ExecutionSequence`
                        (:`then_0`
                          ;[1 1 1] Destroy actor if it's still colliding
                          (`self.Destroy Actor if Still Colliding` (`local.Current Spawned Actor`) (`|MakeArray` (`local.Hit Actor`))))
                        (:`then_1`
                          ;[1 1 1] Move actor to ground
                          (bind _location_2 (`/Game/Blueprints/FunctionLibraries/BPFL_Transform.Get Actor's World Location` (`local.Current Spawned Actor`)))
                          (bind _location_3 (`/Game/Blueprints/FunctionLibraries/BPFL_Transform.Get Actor's World Location` (`self.Prop Parent Actor`)))
                          (`self.Sweep Actor to Point` (`local.Current Spawned Actor`) (`KismetMathLibrary.MakeVector` (.x _location_2) (.y _location_2) (.z _location_3))))
                        (:`then_2`
                          ;[1 1 1] Register Actor
                          (`/Engine/EditorBlueprintResources/StandardMacros.IsValid` (`local.Current Spawned Actor`)
                            (:`Is Valid`
                              (set `Actor.Tags` (`|MakeArray` "Attic Prop" (`KismetStringLibrary.Conv_StringToName` (`KismetSystemLibrary.GetObjectName` (`self.Prop Parent Actor`)))) (`local.Current Spawned Actor`))
                              (`KismetArrayLibrary.Array_Add` (`self.Generated Actors`) (`local.Current Spawned Actor`))
                              (`BlueprintSetLibrary.Set_Add` (`local.Sweep Spawned Actor Set`) (`local.Current Spawned Actor`))
                              (`Actor.K2_AttachToActor` (`local.Current Spawned Actor`) (`self.Prop Parent Actor`) "Props" "KeepWorld" "KeepWorld" "KeepWorld" true)))))))))
              (`Actor.K2_DestroyActor` (`local.Sweep Actor`))))))
      (:`then_3`
        ;[1 1 1] Calculate X- sweep locations
        (for _index_2 (range (+ (`KismetMathLibrary.FTrunc` (* (.y (`local.Spawn Extent`)) 2.0 0.01)) 1))
          (set `local.Ray Index` _index_2)
          (`|ExecutionSequence`
            (:`then_0`
              (`BlueprintSetLibrary.Set_Clear` (`local.Sweep Spawned Actor Set`)))
            (:`then_1`
              ;;[1 1 1] Spawn actor for calculating sweeping
              (set `local.Sweep Actor Class` _outitem_3)
              (bind _returnvalue_3 (`|SpawnActorFromClass` _outitem_3 (`KismetMathLibrary.MakeTransform` (+ (`KismetMathLibrary.GreaterGreater_VectorRotator` (+ (`KismetMathLibrary.MakeVector` 0.0 (+ (`KismetMathLibrary.RandomFloatInRangeFromStream` -25.0 25.0 (`self.Random Stream`)) (* (`local.Ray Index`) 100.0))) (* (1.0 -1.0 0.0) (`local.Spawn Extent`))) (`local.World Rotation`)) (`self.Location`)) (`KismetMathLibrary.ComposeRotators` (`KismetMathLibrary.MakeRotator` 0.0 0.0 180.0) (`local.World Rotation`))) "AlwaysSpawn" "OverrideRootScale" null null))
              (set `local.Sweep Actor` _returnvalue_3))
            (:`then_2`
              ;;[1 1 1] Trace along sweep for hits
              (bind (_origin_2 _extent_2) (`/Game/Blueprints/FunctionLibraries/BPFL_Generation.Get Bounds For Generative Actor` (`local.Sweep Actor`)))
              (bind _outhits_2 (`KismetSystemLibrary.BoxTraceMultiForObjects` _origin_2 (+ _origin_2 (`KismetMathLibrary.GreaterGreater_VectorRotator` (+ (* (`local.Spawn Extent`) (-2.0 0.0 0.0)) (-100.0 0.0 0.0)) (`local.World Rotation`))) (- _extent_2 (2.0 2.0 2.0)) (struct) (`|MakeArray` "ObjectTypeQuery1" :!type "EObjectTypeQuery Enum") false (`|MakeArray` (`local.Sweep Actor`)) (`local.Draw Debug Type`)))
              (set `local.Sweep Hit Array` _outhits_2)
              (goto _label)))))
      (:`then_4`
        ;[1 1 1] Calculate Y+ sweep locations
        (for _index_3 (range (+ (`KismetMathLibrary.FTrunc` (* (.x (`local.Spawn Extent`)) 2.0 0.01)) 1))
          (set `local.Ray Index` _index_3)
          (`|ExecutionSequence`
            (:`then_0`
              (`BlueprintSetLibrary.Set_Clear` (`local.Sweep Spawned Actor Set`)))
            (:`then_1`
              ;;[1 1 1] Spawn actor for calculating sweeping
              (set `local.Sweep Actor Class` _outitem_4)
              (bind _returnvalue_4 (`|SpawnActorFromClass` _outitem_4 (`KismetMathLibrary.MakeTransform` (+ (`KismetMathLibrary.GreaterGreater_VectorRotator` (+ (`KismetMathLibrary.MakeVector` (+ (`KismetMathLibrary.RandomFloatInRangeFromStream` -25.0 25.0 (`self.Random Stream`)) (* (`local.Ray Index`) 100.0))) (* (-1.0 -1.0 0.0) (`local.Spawn Extent`))) (`local.World Rotation`)) (`self.Location`)) (`KismetMathLibrary.ComposeRotators` (`KismetMathLibrary.MakeRotator` 0.0 0.0 90.0) (`local.World Rotation`))) "AlwaysSpawn" "OverrideRootScale" null null))
              (set `local.Sweep Actor` _returnvalue_4))
            (:`then_2`
              ;;[1 1 1] Trace along sweep for hits
              (bind (_origin_3 _extent_3) (`/Game/Blueprints/FunctionLibraries/BPFL_Generation.Get Bounds For Generative Actor` (`local.Sweep Actor`)))
              (bind _outhits_3 (`KismetSystemLibrary.BoxTraceMultiForObjects` _origin_3 (+ _origin_3 (`KismetMathLibrary.GreaterGreater_VectorRotator` (+ (* (`local.Spawn Extent`) (0.0 2.0 0.0)) (0.0 100.0 0.0)) (`local.World Rotation`))) (- _extent_3 (2.0 2.0 2.0)) (struct) (`|MakeArray` "ObjectTypeQuery1" :!type "EObjectTypeQuery Enum") false (`|MakeArray` (`local.Sweep Actor`)) (`local.Draw Debug Type`)))
              (set `local.Sweep Hit Array` _outhits_3)
              (goto _label)))))
      (:`then_5`
        ;[1 1 1] Calculate Y- sweep locations
        (for _index_4 (range (+ (`KismetMathLibrary.FTrunc` (* (.x (`local.Spawn Extent`)) 2.0 0.01)) 1))
          (set `local.Ray Index` _index_4)
          (`|ExecutionSequence`
            (:`then_0`
              (`BlueprintSetLibrary.Set_Clear` (`local.Sweep Spawned Actor Set`)))
            (:`then_1`
              ;;[1 1 1] Spawn actor for calculating sweeping
              (set `local.Sweep Actor Class` _outitem)
              (bind _returnvalue_5 (`|SpawnActorFromClass` _outitem (`KismetMathLibrary.MakeTransform` (+ (`KismetMathLibrary.GreaterGreater_VectorRotator` (+ (`KismetMathLibrary.MakeVector` (+ (`KismetMathLibrary.RandomFloatInRangeFromStream` -25.0 25.0 (`self.Random Stream`)) (* (`local.Ray Index`) 100.0))) (* (-1.0 1.0 0.0) (`local.Spawn Extent`))) (`local.World Rotation`)) (`self.Location`)) (`KismetMathLibrary.ComposeRotators` (`KismetMathLibrary.MakeRotator` 0.0 0.0 270.0) (`local.World Rotation`))) "AlwaysSpawn" "OverrideRootScale" null null))
              (set `local.Sweep Actor` _returnvalue_5))
            (:`then_2`
              ;;[1 1 1] Trace along sweep for hits
              (bind (_origin_4 _extent_4) (`/Game/Blueprints/FunctionLibraries/BPFL_Generation.Get Bounds For Generative Actor` (`local.Sweep Actor`)))
              (bind _outhits_4 (`KismetSystemLibrary.BoxTraceMultiForObjects` _origin_4 (+ _origin_4 (`KismetMathLibrary.GreaterGreater_VectorRotator` (+ (* (`local.Spawn Extent`) (0.0 -2.0 0.0)) (0.0 -100.0 0.0)) (`local.World Rotation`))) (- _extent_4 (2.0 2.0 2.0)) (struct) (`|MakeArray` "ObjectTypeQuery1" :!type "EObjectTypeQuery Enum") false (`|MakeArray` (`local.Sweep Actor`)) (`local.Draw Debug Type`)))
              (set `local.Sweep Hit Array` _outhits_4)
              (goto _label))))))
    (else
      (`KismetSystemLibrary.PrintString` (`KismetStringLibrary.Concat_StrStr` "No spawnable props for " (`KismetSystemLibrary.GetDisplayName` self))))))