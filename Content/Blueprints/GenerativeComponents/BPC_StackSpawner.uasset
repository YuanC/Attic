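; Generative component, named as a stack spawner, that currently spawns a single random prop under a parent actor.
; Generate picks a random class from Meshes, spawns it at a fixed offset unless collision cannot be resolved, and records it in GeneratedActors.
; The spawned actor is attached to PropParentActor with relative rules; an empty Meshes list prints a warning instead.
; No stacking logic is present.
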(fn `Generate`
  (if (`KismetArrayLibrary.Array_IsNotEmpty` (`self.Meshes`))
    (`|ExecutionSequence`
      (:`then_0`
        (bind _returnvalue (`|SpawnActorFromClass` (`KismetArrayLibrary.Array_Random` (`self.Meshes`)) (`KismetMathLibrary.MakeTransform` (0.0 -50.0 0.0)) (enumliteral `ESpawnActorCollisionHandlingMethod` "AdjustIfPossibleButDontSpawnIfColliding") "OverrideRootScale" null null))
        (`KismetArrayLibrary.Array_Add` (`self.Generated Actors`) _returnvalue)
        (`Actor.K2_AttachToActor` _returnvalue (`self.Prop Parent Actor`) "None" "KeepRelative" "KeepRelative" "KeepRelative" true)))
    (else
      (`KismetSystemLibrary.PrintString` (`KismetStringLibrary.Concat_StrStr` (`KismetSystemLibrary.GetDisplayName` self) " has no meshes to spawn")))))