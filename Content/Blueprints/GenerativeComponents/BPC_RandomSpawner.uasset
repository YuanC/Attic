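; Random prop spawner component that scatters props from SpawnableProps inside a box for procedural generation of attic props.
; Generate derives the attempt count from box area and PropDensity, then picks class, position and yaw from a seeded RandomStream.
; Each spawn runs its own generative initialization, then a WorldStatic box overlap test with configurable ignored actors.
; Overlapping props are destroyed; survivors are tagged, recorded and attached to PropParentActor, with optional debug boxes.
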(fn `Generate`
  (locals (`Spawn Location` :type "Vector Structure") (`Current Spawned Actor` :type "Actor Object Reference") (`Ignored Actors` :type "Array of Actor Object Reference") (`Spawned Actor Location` :type "Vector Structure") (`Spawned Actor Extent` :type "Vector Structure") (`Is Spawned Actor Generative` :type Boolean))
  (if (`self.Show Debug Spawn Points`)
    (`KismetSystemLibrary.DrawDebugBox` (+ (`self.Location`) (`Actor.K2_GetActorLocation` (`self.Prop Parent Actor`))) (`self.Extent`) (struct :`R` 0.17984 :`B` 0.401042 :`A` 1.0) (struct) 10.0 20.0))
  (if (`KismetArrayLibrary.Array_IsNotEmpty` (`self.Spawnable Props`))
    ;[1 1 1] Choose random position in bounds
    (for _ (range (+ (`KismetMathLibrary.FTrunc` (* (.x (/ (`self.Extent`) (100.0 100.0 100.0))) (.y (/ (`self.Extent`) (100.0 100.0 100.0))) (`self.Prop Density`))) 1))
      (bind _point (`/Game/Blueprints/FunctionLibraries/BPFL_DeterministicRandom.RandomPointInBoundingBox` (`self.Random Stream`) (`self.Location`) (`self.Extent`)))
      ;[1 1 1] Spawn actor at location
      (set `local.Spawn Location` _point)
      (bind _returnvalue (`|SpawnActorFromClass` (`KismetArrayLibrary.Array_RandomFromStream` (`self.Spawnable Props`) (`self.Random Stream`)) (`KismetMathLibrary.MakeTransform` (`local.Spawn Location`) (`KismetMathLibrary.MakeRotator` 0.0 0.0 (`KismetMathLibrary.RandomFloatInRangeFromStream` 0.0 360.0 (`self.Random Stream`)))) "Undefined" "OverrideRootScale" null null))
      (bind _output_get (set `local.Current Spawned Actor` _returnvalue))
      (if (`KismetSystemLibrary.IsValid` _output_get)
        (`|ExecutionSequence`
          (:`then_0`
            ;[1 1 1] Call prop generation functions
            (`/Game/Blueprints/FunctionLibraries/BPFL_Generation.Initialize Generative Prop` (`local.Current Spawned Actor`) (`self.Prop Parent Actor`) (`self.Random Stream`) (`self.Dirtiness`) (`self.Prop Density`) (`self.Show Debug Spawn Points`)))
          (:`then_1`
            ;[1 1 1] Configure collisions to ignore
            (if (`self.Handle Collision`)
              (set `local.Ignored Actors` (`|MakeArray` (`local.Current Spawned Actor`)))
              (if (`self.Ignore Parent Collision`)
                (`KismetArrayLibrary.Array_Add` (`local.Ignored Actors`) (`self.Prop Parent Actor`))
                (if (`self.Ignore Collision With ActorsFrom Same Spawner`)
                  (`KismetArrayLibrary.Array_Append` (`local.Ignored Actors`) (`self.Generated Actors`))))))
          (:`then_2`
            ;[1 1 1] Remove mesh based on collisions
            (bind (_origin _extent _is_generative_prop) (`/Game/Blueprints/FunctionLibraries/BPFL_Generation.Get Bounds For Generative Actor` (`local.Current Spawned Actor`)))
            (set `local.Spawned Actor Location` (+ _origin (0.0 0.0 2.0)))
            (set `local.Spawned Actor Extent` (+ _extent (0.0 0.0 -2.0)))
            (set `local.Is Spawned Actor Generative` _is_generative_prop)
            (bind _outactors (`KismetSystemLibrary.BoxOverlapActors` (`local.Spawned Actor Location`) (`local.Spawned Actor Extent`) (`|MakeArray` "ObjectTypeQuery1" :!type "EObjectTypeQuery Enum") null (`local.Ignored Actors`)))
            (if (`KismetArrayLibrary.Array_IsEmpty` _outactors)
              (if (`self.Show Debug Spawn Points`)
                (if (`local.Is Spawned Actor Generative`)
                  (`KismetSystemLibrary.DrawDebugBox` (`local.Spawned Actor Location`) (`local.Spawned Actor Extent`) (struct :`G` 1.0 :`B` 0.983632 :`A` 1.0) (struct) 10.0 0.5)
                  (else
                    (`KismetSystemLibrary.DrawDebugBox` (`local.Spawned Actor Location`) (`local.Spawned Actor Extent`) (struct :`R` 0.432467 :`G` 1.0 :`B` 0.426326 :`A` 1.0) (struct) 10.0 0.5))))
              ;[1 1 1] Register mesh
              (set `Actor.Tags` (`|MakeArray` "Attic Prop" (`KismetStringLibrary.Conv_StringToName` (`KismetSystemLibrary.GetObjectName` (`self.Prop Parent Actor`)))) (`local.Current Spawned Actor`))
              (`KismetArrayLibrary.Array_Add` (`self.Generated Actors`) (`local.Current Spawned Actor`))
              (`Actor.K2_AttachToActor` (`local.Current Spawned Actor`) (`self.Prop Parent Actor`) "Props" "KeepWorld" "KeepWorld" "KeepWorld" true)
              (else
                (`Actor.K2_DestroyActor` (`local.Current Spawned Actor`))
                (`KismetSystemLibrary.DrawDebugBox` (`local.Spawned Actor Location`) (`local.Spawned Actor Extent`) (struct :`R` 0.058824 :`G` 0.015686 :`B` 0.019608 :`A` 1.0) (struct) 10.0 0.5)
                (`KismetSystemLibrary.PrintString` "HI")))))))
    (else
      (`KismetSystemLibrary.PrintString` (`KismetStringLibrary.Concat_StrStr` "No spawnable props for " (`KismetSystemLibrary.GetDisplayName` self))))))