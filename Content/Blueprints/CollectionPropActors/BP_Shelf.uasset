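; BP_Shelf is a prop actor meant to generate a randomly sized shelf.
; Generate picks width and height up to configured maximums from a random stream, then adds a random spawner component once per row.
; The work appears unfinished: the per-column loop is empty, the construction script does nothing, and the event graph's GenerateShelf call is never executed.
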(fn `Generate`
  (`|ExecutionSequence`
    (:`then_0`
      ;[1 1 1] Set dimensions
      (set `self.Width` (`KismetMathLibrary.RandomIntegerInRangeFromStream` 1 (`self.Max Width`) (`self.Random Stream`)))
      (set `self.Height` (`KismetMathLibrary.RandomIntegerInRangeFromStream` 1 (`self.Max Height`) (`self.Random Stream`))))
    (:`then_1`
      (for _ (range 1 (+ (`self.Height`) 1))
        (`|ExecutionSequence`
          (:`then_0`
            (for _ (range 1 (+ (`self.Width`) 1))
              _))
          (:`then_1`
            (`AddComponent|NODE_AddBPC_RandomSpawner-0`)))))))

(fn `UserConstructionScript`)