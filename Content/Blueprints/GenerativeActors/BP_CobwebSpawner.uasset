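; Generative actor that spawns cobweb props over an area sized by its length and width in meters.
; Generate clears previous output, resets the BPCCobwebSpawner component, then passes it dirtiness, density, random stream, debug flag, location, half-size extent and any prop list override.
; After the component generates, the actor derives a new random stream from the current one.
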(fn `Generate`
  (`parent.Generate`)
  (`|ExecutionSequence`
    (:`then_0`
      (`self.Remove`))
    (:`then_1`
      ;[1 1 1] Reset and regenerate spawners
      (`|ExecutionSequence`
        (:`then_0`
          (`/Game/Blueprints/GenerativeComponents/BPC_GenerativeComponent.Reset` (`self.BPC_CobwebSpawner`)))
        (:`then_1`
          ;[1 1 1] Set spawning parameters
          (`|ExecutionSequence`
            (:`then_0`
              (set `/Game/Blueprints/GenerativeComponents/BPC_GenerativeComponent.Prop Parent Actor` self (`self.BPC_CobwebSpawner`)))
            (:`then_1`
              (set `/Game/Blueprints/GenerativeComponents/BPC_GenerativeComponent.Dirtiness` (`self.Dirtiness`) (`self.BPC_CobwebSpawner`)))
            (:`then_2`
              (set `/Game/Blueprints/GenerativeComponents/BPC_GenerativeComponent.Random Stream` (`self.Random Stream`) (`self.BPC_CobwebSpawner`)))
            (:`then_3`
              (set `/Game/Blueprints/GenerativeComponents/BPC_GenerativeComponent.Prop Density` (`self.Prop Density`) (`self.BPC_CobwebSpawner`)))
            (:`then_4`
              (set `/Game/Blueprints/GenerativeComponents/BPC_GenerativeComponent.Show Debug Spawn Points` (`self.Show Debug Spawn Points`) (`self.BPC_CobwebSpawner`)))
            (:`then_5`
              (if (`KismetArrayLibrary.Array_IsNotEmpty` (`self.Spawnable Props`))
                (set `/Game/Blueprints/GenerativeComponents/BPC_CobwebSpawner.Spawnable Props` (`self.Spawnable Props`) (`self.BPC_CobwebSpawner`))))
            (:`then_6`
              (set `/Game/Blueprints/GenerativeComponents/BPC_GenerativeComponent.Location` (`/Game/Blueprints/FunctionLibraries/BPML_Transform.GetActorWorldLocation` self) (`self.BPC_CobwebSpawner`)))
            (:`then_7`
              (bind _returnvalue (`/Game/Blueprints/FunctionLibraries/BPFL_Vectors.Make Centimeter Vector From Meters` (`KismetMathLibrary.Conv_IntToDouble` (`self.Length`)) (`KismetMathLibrary.Conv_IntToDouble` (`self.Width`))))
              (set `/Game/Blueprints/GenerativeComponents/BPC_GenerativeComponent.Extent` (/ _returnvalue (2.0 2.0 1.0)) (`self.BPC_CobwebSpawner`)))))
        (:`then_2`
          (`/Game/Blueprints/GenerativeComponents/BPC_GenerativeComponent.Generate` (`self.BPC_CobwebSpawner`)))
        (:`then_3`
          (set `self.Random Stream` (`KismetMathLibrary.MakeRandomStream` (`KismetMathLibrary.RandomIntegerFromStream` 10000 (`self.Random Stream`)))))))))

(fn `UserConstructionScript`
  (`parent.UserConstructionScript`))