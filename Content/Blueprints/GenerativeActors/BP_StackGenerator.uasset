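; Generative actor that builds seeded random stacks of attic props in a grid of fixed or random width, height and depth.
; Generate clears old props, then spawns and initializes each with random yaw, thinning upper layers by HeightFalloff.
; Props are placed relative to earlier ones, pushed out of collisions or destroyed, then swept down and optionally toward the center.
; Survivors are tagged, attached and recorded for GetBounds.
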(fn `Generate`
  (locals (`Instance X` :type Integer) (`Instance Y` :type Integer) (`Instance Z` :type Integer) (`Current Spawned Actor` :type "Actor Object Reference") (`Previous Spawned Z Actor` :type "Actor Object Reference") (`Previous Spawned Y Actor` :type "Actor Object Reference") (`Previous Spawned Y- Actor` :type "Actor Object Reference") (`Previous Spawned X Actor` :type "Actor Object Reference") (`Previous Spawned X- Actor` :type "Actor Object Reference"))
  (bind _current_spawned_actor (`local.Current Spawned Actor`))
  (bind _current_spawned_actor_2 (`local.Current Spawned Actor`))
  (bind _returnvalue (`KismetMathLibrary.GreaterGreater_VectorRotator` (`KismetMathLibrary.MakeVector` 0.0 (* (`self.Gap Between Actors`) (`KismetMathLibrary.Conv_IntToDouble` (+ (* (mod (`local.Instance Y`) 2) -2) 1)))) (`/Game/Blueprints/FunctionLibraries/BPML_Transform.GetActorWorldRotation` self)))
  (bind _returnvalue_2 (`KismetMathLibrary.GreaterGreater_VectorRotator` (`KismetMathLibrary.MakeVector` (* (`self.Gap Between Actors`) (`KismetMathLibrary.Conv_IntToDouble` (+ (* (mod (`local.Instance X`) 2) -2) 1)))) (`/Game/Blueprints/FunctionLibraries/BPML_Transform.GetActorWorldRotation` self)))
  (`parent.Generate`)
  (`|ExecutionSequence`
    (:`then_0`
      (`self.Remove`))
    (:`then_1`
      ;[1 1 1] Set dimensions
      (if (`self.Set To Max Dimensions`)
        (set `self.Width` (`self.Max Width`))
        (set `self.Height` (`self.Max Height`))
        (set `self.Depth` (`self.Max Depth`))
        (else
          (set `self.Width` (`KismetMathLibrary.RandomIntegerInRangeFromStream` 1 (`self.Max Width`) (`self.Random Stream`)))
          (set `self.Height` (`KismetMathLibrary.RandomIntegerInRangeFromStream` 1 (`self.Max Height`) (`self.Random Stream`)))
          (set `self.Depth` (`KismetMathLibrary.RandomIntegerInRangeFromStream` 1 (`self.Max Depth`) (`self.Random Stream`))))))
    (:`then_2`
      (if (`KismetArrayLibrary.Array_IsNotEmpty` (`self.Spawnable Props`))
        ;[1 1 1] Loop through spawn positions
        (for _index (range 1 (+ (`self.Depth`) 1))
          (set `local.Instance X` _index)
          (for _index_2 (range 1 (+ (`self.Width`) 1))
            (set `local.Instance Y` _index_2)
            (for _index_3 (range 1 (+ (`self.Height`) 1))
              (set `local.Instance Z` _index_3)
              (`|ExecutionSequence`
                (:`then_0`
                  (if (> (`local.Instance Z`) 1)
                    (if (not (> (`KismetMathLibrary.RandomFloatInRangeFromStream` 0.01 1.0 (`self.Random Stream`)) (`self.Height Falloff`)))
                      (break))))
                (:`then_1`
                  ;[1 1 1] Spawn actor
                  (bind _returnvalue_3 (`|SpawnActorFromClass` (`KismetArrayLibrary.Array_RandomFromStream` (`self.Spawnable Props`) (`self.Random Stream`)) (`KismetMathLibrary.MakeTransform` (0.0 0.0 0.0) (`KismetMathLibrary.MakeRotator` 0.0 0.0 (`KismetMathLibrary.RandomFloatInRangeFromStream` 0.0 (* (`self.Rotation Variability`) 360.0) (`self.Random Stream`)))) "AlwaysSpawn" "OverrideRootScale" null null))
                  (bind _output_get (set `local.Current Spawned Actor` _returnvalue_3))
                  (if (`KismetSystemLibrary.IsValid` _output_get)
                    (`|ExecutionSequence`
                      (:`then_0`
                        ;[1 1 1] Generate actor
                        (`/Game/Blueprints/FunctionLibraries/BPFL_Generation.Initialize Generative Prop` (`local.Current Spawned Actor`) self (`self.Random Stream`) (`self.Dirtiness`) (`self.Prop Density`) (`self.Show Debug Spawn Points`)))
                      (:`then_1`
                        ;[1 1 1] Naively move to expected location, based on bounds of spawned actor and previous spawned actor
                        (`/Engine/EditorBlueprintResources/StandardMacros.IsValid` (`local.Previous Spawned Z Actor`)
                          (:`Is Valid`
                            (if (> (`local.Instance Z`) 1)
                              ;;[1 1 1] Spawn on top of previous actor
                              (`self.K2_SetActorLocation` (`local.Current Spawned Actor`) (+ (`/Game/Blueprints/FunctionLibraries/BPML_Transform.GetActorWorldLocation` (`local.Previous Spawned Z Actor`)) (0.0 0.0 1.0)) false false)
                              (`self.Uncollide Actor on Z` (`local.Current Spawned Actor`) (`local.Previous Spawned Z Actor`))
                              (elif (> (`local.Instance Y`) 1)
                                ;;[1 1 1] Shift actor to start a new row on Y axis
                                (if (== (mod (`local.Instance Y`) 2) 0)
                                  (`self.K2_SetActorLocation` (`local.Current Spawned Actor`) (+ (`/Game/Blueprints/FunctionLibraries/BPML_Transform.GetActorWorldLocation` (`local.Previous Spawned Y Actor`)) _returnvalue) false false)
                                  (else
                                    (`self.K2_SetActorLocation` (`local.Current Spawned Actor`) (+ (`/Game/Blueprints/FunctionLibraries/BPML_Transform.GetActorWorldLocation` (`local.Previous Spawned Y- Actor`)) _returnvalue) false false)))
                                (else
                                  ;;[1 1 1] Shift actor to start a new row on X axis
                                  (if (== (mod (`local.Instance X`) 2) 0)
                                    (`self.K2_SetActorLocation` (`local.Current Spawned Actor`) (+ (`/Game/Blueprints/FunctionLibraries/BPML_Transform.GetActorWorldLocation` (`local.Previous Spawned X Actor`)) _returnvalue_2) false false)
                                    (else
                                      (`self.K2_SetActorLocation` (`local.Current Spawned Actor`) (+ _returnvalue_2 (`/Game/Blueprints/FunctionLibraries/BPML_Transform.GetActorWorldLocation` (`local.Previous Spawned X- Actor`))) false false)))))))
                          (:`Is Not Valid`
                            ;;[1 1 1] Spawn First Actor
                            (`self.K2_SetActorLocation` (`local.Current Spawned Actor`) (`/Game/Blueprints/FunctionLibraries/BPML_Transform.GetActorWorldLocation` self) false false))))
                      (:`then_2`
                        ;[1 1 1] Attempt to adjust for collisions
                        (`self.Uncollide Actor by X` (`local.Current Spawned Actor`))
                        (`self.Uncollide Actor by Y` (`local.Current Spawned Actor`)))
                      (:`then_3`
                        ;[1 1 1] Destroy actor if it's still colliding
                        (bind _is_actor_destroyed (`self.Destoy Actor if Colliding` (`local.Current Spawned Actor`)))
                        (if _is_actor_destroyed
                          _))
                      (:`then_4`
                        (`/Engine/EditorBlueprintResources/StandardMacros.IsValid` (`local.Current Spawned Actor`)
                          (:`Is Valid`
                            (`|ExecutionSequence`
                              (:`then_0`
                                ;[1 1 1] Attempt to move actor as close to the center of the stack as possible
                                (`self.Sweep Actor to Point` _current_spawned_actor_2 (`KismetMathLibrary.MakeVector` (.x (`/Game/Blueprints/FunctionLibraries/BPML_Transform.GetActorWorldLocation` _current_spawned_actor_2)) (.y (`/Game/Blueprints/FunctionLibraries/BPML_Transform.GetActorWorldLocation` _current_spawned_actor_2)) (.z (`/Game/Blueprints/FunctionLibraries/BPML_Transform.GetActorWorldLocation` self))))
                                (if (`self.Cluster Actors Together`)
                                  (`self.Sweep Actor to Point` _current_spawned_actor (`KismetMathLibrary.MakeVector` (.x (`/Game/Blueprints/FunctionLibraries/BPML_Transform.GetActorWorldLocation` self)) (.y (`/Game/Blueprints/FunctionLibraries/BPML_Transform.GetActorWorldLocation` self)) (.z (`/Game/Blueprints/FunctionLibraries/BPML_Transform.GetActorWorldLocation` _current_spawned_actor))))))
                              (:`then_1`
                                ;[1 1 1] Register Actor
                                (set `Actor.Tags` (`|MakeArray` "Attic Prop" (`KismetStringLibrary.Conv_StringToName` (`KismetSystemLibrary.GetObjectName` self))) (`local.Current Spawned Actor`))
                                (`KismetArrayLibrary.Array_Add` (`self.Generated Actors`) (`local.Current Spawned Actor`))
                                (`self.K2_AttachToActor` (`local.Current Spawned Actor`) self "Props" "KeepWorld" "KeepWorld" "KeepWorld" true))
                              (:`then_2`
                                ;[1 1 1] Store previously spawned actors to calculate the next iteration's location
                                (`|ExecutionSequence`
                                  (:`then_0`
                                    (set `local.Previous Spawned Z Actor` (`local.Current Spawned Actor`)))
                                  (:`then_1`
                                    (if (== (`local.Instance Z`) 1)
                                      (if (== (`local.Instance Y`) 1)
                                        (bind _output_get_2 (set `local.Previous Spawned Y Actor` (`local.Current Spawned Actor`)))
                                        (set `local.Previous Spawned Y- Actor` _output_get_2)
                                        (if (== (`local.Instance X`) 1)
                                          (bind _output_get_3 (set `local.Previous Spawned X Actor` (`local.Current Spawned Actor`)))
                                          (set `local.Previous Spawned X- Actor` _output_get_3)
                                          (elif (== (mod (`local.Instance X`) 2) 0)
                                            (set `local.Previous Spawned X Actor` (`local.Current Spawned Actor`))
                                            (else
                                              (set `local.Previous Spawned X- Actor` (`local.Current Spawned Actor`)))))
                                        (elif (== (mod (`local.Instance Y`) 2) 0)
                                          (set `local.Previous Spawned Y Actor` (`local.Current Spawned Actor`))
                                          (else
                                            (set `local.Previous Spawned Y- Actor` (`local.Current Spawned Actor`))))))))))))))))))))
        (else
          (`KismetSystemLibrary.PrintString` (`KismetStringLibrary.Concat_StrStr` "No spawnable props for " (`KismetSystemLibrary.GetDisplayName` self))))))))

(fn `GetBounds`
  (returns (Origin :type "Vector Structure") (BoxExtent :type "Vector Structure"))
  (bind (_center _boxextent) (`GameplayStatics.GetActorArrayBounds` (`self.Generated Actors`) true))
  (return _center _boxextent))

(fn `Remove`
  (`parent.Remove`))

(fn `UserConstructionScript`)