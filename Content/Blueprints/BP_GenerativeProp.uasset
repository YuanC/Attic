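; Base Blueprint for procedurally generated props, regenerated from the construction script when automatic regeneration is enabled.
; Generate optionally seeds a random stream, then calls OverrideVariables, an empty hook; GenerateRandom rerolls the seed first.
; Remove targets child actors and those tagged with this prop's name plus "Attic Prop".
; Bounds-based helpers resolve placement by nudging actors along axes, destroying overlapping ones or box-sweeping them to target points.
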(fn `Destoy Actor if Colliding`
  (params (`Actor to destroy` :type "Actor Object Reference (by ref)"))
  (returns (`Is Actor Destroyed` :type Boolean))
  (bind (_origin _extent) (`/Game/Blueprints/FunctionLibraries/BPFL_Generation.Get Bounds For Generative Actor` `Actor to destroy`))
  (bind (_outactors _returnvalue) (`KismetSystemLibrary.BoxOverlapActors` _origin _extent (`|MakeArray` "ObjectTypeQuery1" :!type "EObjectTypeQuery Enum") null (`|MakeArray` `Actor to destroy`)))
  (if _returnvalue
    (`self.K2_DestroyActor` `Actor to destroy`))
  (return _returnvalue))

(fn `Generate`
  (if (`self.Use Random Seed`)
    (`KismetMathLibrary.SetRandomStreamSeed` (`self.Random Stream`) (`self.Random Seed`)))
  (`self.Override Variables`))

(fn `Generate Random`
  (set `self.Random Seed` (`KismetMathLibrary.RandomInteger` 1000000))
  (set `self.Use Random Seed` true)
  (`self.Generate`))

(fn `GetBounds`
  (returns (Origin :type "Vector Structure") (BoxExtent :type "Vector Structure"))
  (bind (_origin _boxextent) (`self.GetActorBounds` true true))
  (return _origin _boxextent))

(fn `Override Variables`)

(fn `Remove`
  (bind _childactors (`self.GetAllChildActors` true))
  (bind _output (`|GetArrayItem` _childactors))
  (`|ExecutionSequence`
    (:`then_0`
      ;[1 1 1] Remove associated actors
      (while (`KismetArrayLibrary.Array_IsNotEmpty` _childactors)
        (if (not (`KismetSystemLibrary.IsValid` _output))
          (`self.K2_DestroyActor` _output))))
    (:`then_1`
      (bind _outactors (`GameplayStatics.GetAllActorsWithTag` (`KismetStringLibrary.Conv_StringToName` (`KismetSystemLibrary.GetObjectName` self))))
      (for _array_element _outactors
        (if (and (`self.ActorHasTag` _array_element "Attic Prop") (`KismetSystemLibrary.IsValid` _array_element))
          (`self.K2_DestroyActor` _array_element))))))

(fn `Sweep Actor to Point`
  (params (`Actor to move` :type "Actor Object Reference (by ref)") (`Target Point` :type "Vector Structure (by ref)"))
  (bind _returnvalue (`/Game/Blueprints/FunctionLibraries/BPML_Transform.GetActorWorldLocation` `Actor to move`))
  (bind (_origin _extent) (`/Game/Blueprints/FunctionLibraries/BPFL_Generation.Get Bounds For Generative Actor` `Actor to move`))
  (bind (_outhit _returnvalue_2) (`KismetSystemLibrary.BoxTraceSingleForObjects` _origin (+ (- _origin _returnvalue) `Target Point`) _extent (struct) (`|MakeArray` "ObjectTypeQuery1" :!type "EObjectTypeQuery Enum") false (`|MakeArray` `Actor to move`) "None" false))
  (if _returnvalue_2
    (`self.K2_SetActorLocation` `Actor to move` (+ (`.Location` (`GameplayStatics.BreakHitResult` _outhit)) (- _returnvalue _origin)) true false)
    (else
      (`self.K2_SetActorLocation` `Actor to move` `Target Point` true false)))
  (return))

(fn `Uncollide Actor by X`
  (params (`Actor to move` :type "Actor Object Reference (by ref)"))
  (bind (_origin _extent) (`/Game/Blueprints/FunctionLibraries/BPFL_Generation.Get Bounds For Generative Actor` `Actor to move`))
  (bind (_outhit _returnvalue) (`KismetSystemLibrary.BoxTraceSingleForObjects` _origin _origin _extent (struct) (`|MakeArray` "ObjectTypeQuery1" :!type "EObjectTypeQuery Enum") false (`|MakeArray` `Actor to move`) "None" false))
  (if _returnvalue
    (bind (_origin_2 _extent_2) (`/Game/Blueprints/FunctionLibraries/BPFL_Generation.Get Bounds For Generative Actor` (`.HitActor` (`GameplayStatics.BreakHitResult` _outhit))))
    (bind _returnvalue_2 (* (+ _origin_2 _extent_2 (`KismetMathLibrary.NegateVector` _origin) _extent) (1.0 0.0 0.0)))
    (`self.K2_SetActorLocation` `Actor to move` (+ (`/Game/Blueprints/FunctionLibraries/BPML_Transform.GetActorWorldLocation` `Actor to move`) _returnvalue_2 (* (`KismetMathLibrary.Vector_GetSignVector` _returnvalue_2) (2.0 0.0 0.0))) false false))
  (return))

(fn `Uncollide Actor by Y`
  (params (`Actor to move` :type "Actor Object Reference (by ref)"))
  (bind (_origin _extent) (`/Game/Blueprints/FunctionLibraries/BPFL_Generation.Get Bounds For Generative Actor` `Actor to move`))
  (bind (_outhit _returnvalue) (`KismetSystemLibrary.BoxTraceSingleForObjects` _origin _origin _extent (struct) (`|MakeArray` "ObjectTypeQuery1" :!type "EObjectTypeQuery Enum") false (`|MakeArray` `Actor to move`) "None" false))
  (if _returnvalue
    (bind (_origin_2 _extent_2) (`/Game/Blueprints/FunctionLibraries/BPFL_Generation.Get Bounds For Generative Actor` (`.HitActor` (`GameplayStatics.BreakHitResult` _outhit))))
    (bind _returnvalue_2 (* (+ _origin_2 _extent_2 (`KismetMathLibrary.NegateVector` _origin) _extent) (0.0 1.0 0.0)))
    (`self.K2_SetActorLocation` `Actor to move` (+ (`/Game/Blueprints/FunctionLibraries/BPML_Transform.GetActorWorldLocation` `Actor to move`) _returnvalue_2 (* (`KismetMathLibrary.Vector_GetSignVector` _returnvalue_2) (0.0 2.0 0.0))) false false))
  (return))

(fn `Uncollide Actor on Z`
  (params (`Actor to move` :type "Actor Object Reference (by ref)") (`Colliding actor` :type "Actor Object Reference (by ref)"))
  (bind (_origin _extent) (`/Game/Blueprints/FunctionLibraries/BPFL_Generation.Get Bounds For Generative Actor` `Colliding actor`))
  (bind (_origin_2 _extent_2) (`/Game/Blueprints/FunctionLibraries/BPFL_Generation.Get Bounds For Generative Actor` `Actor to move`))
  (`self.K2_SetActorLocation` `Actor to move` (+ (`/Game/Blueprints/FunctionLibraries/BPML_Transform.GetActorWorldLocation` `Actor to move`) (* (+ (`KismetMathLibrary.NegateVector` _origin_2) _extent_2 _origin _extent) (0.0 0.0 1.0)) (0.0 0.0 1.0)) false false)
  (return))

(fn `UserConstructionScript`
  (`KismetSystemLibrary.FlushPersistentDebugLines`)
  (if (`self.Automatically Regenerate On Edit`)
    (`self.Generate`)))