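; Base component for procedural prop generation, with an empty Generate, prop registration that tracks and attaches spawned actors, and Reset to destroy them.
; Placement helpers use bounds-sized box traces against WorldStatic to push an actor clear along X, Y or Z, or sweep it toward a point until blocked.
; Slightly shrunk overlap boxes detect remaining collisions, either destroying the actor or testing hits against a given actor set.
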(fn `Destroy Actor if Still Colliding`
  (params (`Actor to Move` :type "Actor Object Reference (by ref)"))
  (returns (`Is Actor Destroyed` :type Boolean))
  (locals (`Moving Actor` :type "Actor Object Reference"))
  (set `local.Moving Actor` `Actor to Move`)
  (bind (_origin _extent) (`/Game/Blueprints/FunctionLibraries/BPFL_Generation.Get Bounds For Generative Actor` (`local.Moving Actor`)))
  (bind (_outactors _returnvalue) (`KismetSystemLibrary.BoxOverlapActors` _origin (- _extent (2.0 2.0 2.0)) (`|MakeArray` "ObjectTypeQuery1" :!type "EObjectTypeQuery Enum") null (`|MakeArray` (`local.Moving Actor`))))
  (if _returnvalue
    (`Actor.K2_DestroyActor` (`local.Moving Actor`)))
  (return _returnvalue))

(fn `Generate`)

(fn `Is Actor Colliding with Set`
  (params (`Actor to Move` :type "Actor Object Reference (by ref)") (`Set to Check` :type "Set of Actor Object Reference (by ref)"))
  (returns (`Is Actor Colliding` :type Boolean))
  (locals (`Moving Actor` :type "Actor Object Reference") (`Colliding Set` :type "Set of Actor Object Reference") (`Checking Set` :type "Set of Actor Object Reference"))
  (set `local.Moving Actor` `Actor to Move`)
  (set `local.Checking Set` `Set to Check`)
  (bind (_origin _extent) (`/Game/Blueprints/FunctionLibraries/BPFL_Generation.Get Bounds For Generative Actor` (`local.Moving Actor`)))
  (bind (_outactors _returnvalue) (`KismetSystemLibrary.BoxOverlapActors` _origin (- _extent (2.0 2.0 2.0)) (`|MakeArray` "ObjectTypeQuery1" :!type "EObjectTypeQuery Enum") null (`|MakeArray` (`local.Moving Actor`))))
  (if _returnvalue
    (`BlueprintSetLibrary.Set_AddItems` (`local.Colliding Set`) _outactors)
    (bind _result (`BlueprintSetLibrary.Set_Intersection` (`local.Colliding Set`) (`local.Checking Set`)))
    (return (`BlueprintSetLibrary.Set_IsNotEmpty` _result))
    (else
      (return false))))

(fn `Reset`
  (for _array_element (`self.Generated Actors`)
    (if (`KismetSystemLibrary.IsValid` _array_element)
      (`Actor.K2_DestroyActor` _array_element)
      (else
        (return))))
  (set `self.Generated Actors` (`|MakeArray`))
  (return))

(fn `Sweep Actor to Point`
  (params (`Actor to Move` :type "Actor Object Reference (by ref)") (Location :type "Vector Structure (by ref)"))
  (locals (`Moving Actor` :type "Actor Object Reference") (`Ideal Location` :type "Vector Structure"))
  (set `local.Moving Actor` `Actor to Move`)
  (set `local.Ideal Location` Location)
  (bind _location (`/Game/Blueprints/FunctionLibraries/BPFL_Transform.Get Actor's World Location` (`local.Moving Actor`)))
  (bind (_origin _extent) (`/Game/Blueprints/FunctionLibraries/BPFL_Generation.Get Bounds For Generative Actor` (`local.Moving Actor`)))
  (bind (_outhit _returnvalue) (`KismetSystemLibrary.BoxTraceSingleForObjects` _origin (+ (- _origin _location) (`local.Ideal Location`)) (- _extent (3.0 3.0 3.0)) (struct) (`|MakeArray` "ObjectTypeQuery1" :!type "EObjectTypeQuery Enum") false (`|MakeArray` (`local.Moving Actor`)) "None" false))
  (if _returnvalue
    (`Actor.K2_SetActorLocation` (`local.Moving Actor`) (+ (`.Location` (`GameplayStatics.BreakHitResult` _outhit)) (- _location _origin)) false false)
    (else
      (`Actor.K2_SetActorLocation` (`local.Moving Actor`) (`local.Ideal Location`) false false)))
  (return))

(fn `Uncollide Actor on X Axis`
  (params (`Actor to Move` :type "Actor Object Reference (by ref)"))
  (locals (`Moving Actor` :type "Actor Object Reference"))
  (set `local.Moving Actor` `Actor to Move`)
  (bind (_origin _extent) (`/Game/Blueprints/FunctionLibraries/BPFL_Generation.Get Bounds For Generative Actor` (`local.Moving Actor`)))
  (bind (_outhit _returnvalue) (`KismetSystemLibrary.BoxTraceSingleForObjects` _origin _origin _extent (struct) (`|MakeArray` "ObjectTypeQuery1" :!type "EObjectTypeQuery Enum") false (`|MakeArray` (`local.Moving Actor`))))
  (if _returnvalue
    (bind (_origin_2 _extent_2) (`/Game/Blueprints/FunctionLibraries/BPFL_Generation.Get Bounds For Generative Actor` (`.HitActor` (`GameplayStatics.BreakHitResult` _outhit))))
    (bind _location (`/Game/Blueprints/FunctionLibraries/BPFL_Transform.Get Actor's World Location` (`local.Moving Actor`)))
    (bind _returnvalue_2 (* (+ _origin_2 _extent_2 (`KismetMathLibrary.NegateVector` _origin) _extent) (1.0 0.0 0.0)))
    (`Actor.K2_SetActorLocation` (`local.Moving Actor`) (+ _location _returnvalue_2 (* (`KismetMathLibrary.Vector_GetSignVector` _returnvalue_2) (2.0 0.0 0.0))) false false))
  (return))

(fn `Uncollide Actor on Y Axis`
  (params (`Actor to Move` :type "Actor Object Reference (by ref)"))
  (locals (`Moving Actor` :type "Actor Object Reference"))
  (set `local.Moving Actor` `Actor to Move`)
  (bind (_origin _extent) (`/Game/Blueprints/FunctionLibraries/BPFL_Generation.Get Bounds For Generative Actor` (`local.Moving Actor`)))
  (bind (_outhit _returnvalue) (`KismetSystemLibrary.BoxTraceSingleForObjects` _origin _origin _extent (struct) (`|MakeArray` "ObjectTypeQuery1" :!type "EObjectTypeQuery Enum") false (`|MakeArray` (`local.Moving Actor`))))
  (if _returnvalue
    (bind (_origin_2 _extent_2) (`/Game/Blueprints/FunctionLibraries/BPFL_Generation.Get Bounds For Generative Actor` (`.HitActor` (`GameplayStatics.BreakHitResult` _outhit))))
    (bind _location (`/Game/Blueprints/FunctionLibraries/BPFL_Transform.Get Actor's World Location` (`local.Moving Actor`)))
    (bind _returnvalue_2 (* (+ _origin_2 _extent_2 (`KismetMathLibrary.NegateVector` _origin) _extent) (0.0 1.0 0.0)))
    (`Actor.K2_SetActorLocation` (`local.Moving Actor`) (+ _location _returnvalue_2 (* (`KismetMathLibrary.Vector_GetSignVector` _returnvalue_2) (0.0 2.0 0.0))) false false))
  (return))

(fn `Uncollide Actor on Z Axis`
  (params (`Actor to Move` :type "Actor Object Reference (by ref)"))
  (locals (`Moving Actor` :type "Actor Object Reference"))
  (set `local.Moving Actor` `Actor to Move`)
  (bind (_origin _extent) (`/Game/Blueprints/FunctionLibraries/BPFL_Generation.Get Bounds For Generative Actor` (`local.Moving Actor`)))
  (bind (_outhit _returnvalue) (`KismetSystemLibrary.BoxTraceSingleForObjects` _origin _origin _extent (struct) (`|MakeArray` "ObjectTypeQuery1" :!type "EObjectTypeQuery Enum") false (`|MakeArray` (`local.Moving Actor`))))
  (if _returnvalue
    (bind (_origin_2 _extent_2) (`/Game/Blueprints/FunctionLibraries/BPFL_Generation.Get Bounds For Generative Actor` (`.HitActor` (`GameplayStatics.BreakHitResult` _outhit))))
    (bind _location (`/Game/Blueprints/FunctionLibraries/BPFL_Transform.Get Actor's World Location` (`local.Moving Actor`)))
    (bind _returnvalue_2 (* (+ _origin_2 _extent_2 (`KismetMathLibrary.NegateVector` _origin) _extent) (0.0 0.0 1.0)))
    (`Actor.K2_SetActorLocation` (`local.Moving Actor`) (+ _location _returnvalue_2 (* (`KismetMathLibrary.Vector_GetSignVector` _returnvalue_2) (0.0 0.0 2.0))) false false))
  (return))