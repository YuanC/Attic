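; Procedural attic generator that builds a gabled room in the Construction Script from Length and Height in metres.
; Modular panels become instanced static meshes for the floor, stepped sloping sides and mirrored end walls with triangle edges, with optional debug points per instance.
; A dust particle system scales to fit, its spawn rate driven by Dirtiness and attic size.
; Rafters, struts, lights, focal and environmental assets are empty TODO stubs.
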(fn `Generate Back Rafters (TODO)`)

(fn `Generate Back Wall`
  (`|ExecutionSequence`
    (:`then_0`
      (`StaticMeshComponent.SetStaticMesh` (`self.Back Square Panels`) (`self.FrontSquareMesh`))
      (`StaticMeshComponent.SetStaticMesh` (`self.Triangle Right Panels`) (`self.FrontEdgeRightMesh`))
      (`StaticMeshComponent.SetStaticMesh` (`self.Triangle Left Panels`) (`self.FrontEdgeLeftMesh`)))
    (:`then_1`
      (for _index (range (+ (- (`self.Height`) 2) 1))
        (bind _returnvalue (- (* (- (`self.Height`) _index) 2) 3))
        (for _index_2 (range (+ _returnvalue 1))
          (`self.Add Instance At Location` (`self.Make Centimetre Vector From Metres` (- (`KismetMathLibrary.Conv_IntToDouble` (`self.Length`)) 0.5) (- (`KismetMathLibrary.Conv_IntToDouble` (+ _index_2 (* (/ _returnvalue 2) -1))) 0.5) (`KismetMathLibrary.Conv_IntToDouble` _index)) (struct :`Yaw` 180.0) (`self.Back Square Panels`) (struct :`G` 1.0 :`A` 1.0)))))
    (:`then_2`
      (for _index_3 (range (`self.Height`))
        (bind _returnvalue_2 (`self.Make Centimetre Vector From Metres` (- (`KismetMathLibrary.Conv_IntToDouble` (`self.Length`)) 0.5) (- (`KismetMathLibrary.Conv_IntToDouble` (- (`self.Height`) _index_3)) 0.5) (`KismetMathLibrary.Conv_IntToDouble` _index_3)))
        (`self.Add Instance At Location` _returnvalue_2 (struct :`Yaw` 180.0) (`self.Triangle Right Panels`) (struct :`G` 1.0 :`A` 1.0))
        (`self.Add Instance At Location` (* _returnvalue_2 (1.0 -1.0 1.0)) (struct :`Yaw` 180.0) (`self.Triangle Left Panels`) (struct :`G` 1.0 :`A` 1.0))))))

(fn `Generate Dust Particles`
  (bind _height (`self.Height`))
  (bind _returnvalue (`KismetMathLibrary.Conv_IntToDouble` (`self.Length`)))
  (bind _returnvalue_2 (`KismetMathLibrary.Conv_IntToDouble` (`self.Height`)))
  (bind _returnvalue_3 (* _returnvalue_2 2.0))
  ;[1 1 1] Place and Scale particle system so it covers the whole attic area
  (`SceneComponent.K2_SetRelativeTransform` (`self.Dust_Particles`) (`KismetMathLibrary.MakeTransform` (`self.Make Centimetre Vector From Metres` (/ _returnvalue 2.0) 0.0 (/ _returnvalue_2 2.0)) (struct) (/ (`KismetMathLibrary.MakeVector` _returnvalue _returnvalue_3 _returnvalue_3) (4.0 4.0 2.0))) false false)
  ;[1 1 1] Scale the spawn rate with the attic area so the particle density is constant
  (`NiagaraComponent.SetVariableFloat` (`self.Dust_Particles`) "Spawn Rate" (* (`self.Dirtiness`) 0.1 _height _height (`self.Length`))))

(fn `Generate Environmental Assets (TODO)`)

(fn `Generate Floor`
  (bind _returnvalue (- (* (`self.Height`) 2) 1))
  (`|ExecutionSequence`
    (:`then_0`
      ;[1 1 1] Set Meshes
      (`StaticMeshComponent.SetStaticMesh` (`self.Floor Square Panels`) (`self.FloorMesh`)))
    (:`then_1`
      (for _index (range (+ _returnvalue 1))
        (for _index_2 (range (`self.Length`))
          (`self.Add Instance At Location` (`self.Make Centimetre Vector From Metres` (`KismetMathLibrary.Conv_IntToDouble` _index_2) (- (`KismetMathLibrary.Conv_IntToDouble` _index) (/ (`KismetMathLibrary.Conv_IntToDouble` _returnvalue) 2.0))) (struct) (`self.Floor Square Panels`) (struct :`G` 1.0 :`B` 1.0 :`A` 1.0)))))))

(fn `Generate Focal Assets (TODO)`)

(fn `Generate Front Rafters (TODO)`)

(fn `Generate Front Wall`
  (`|ExecutionSequence`
    (:`then_0`
      ;[1 1 1] Set Meshes
      (`StaticMeshComponent.SetStaticMesh` (`self.Front Square Panels`) (`self.FrontSquareMesh`))
      (`StaticMeshComponent.SetStaticMesh` (`self.Triangle Right Panels`) (`self.FrontEdgeRightMesh`))
      (`StaticMeshComponent.SetStaticMesh` (`self.Triangle Left Panels`) (`self.FrontEdgeLeftMesh`)))
    (:`then_1`
      (for _index (range (+ (- (`self.Height`) 2) 1))
        (bind _returnvalue (- (* (- (`self.Height`) _index) 2) 3))
        (for _index_2 (range (+ _returnvalue 1))
          (`self.Add Instance At Location` (`self.Make Centimetre Vector From Metres` -0.5 (- (`KismetMathLibrary.Conv_IntToDouble` (+ _index_2 (* (/ _returnvalue 2) -1))) 0.5) (`KismetMathLibrary.Conv_IntToDouble` _index)) (struct) (`self.Front Square Panels`) (struct :`G` 1.0 :`A` 1.0)))))
    (:`then_2`
      (for _index_3 (range (`self.Height`))
        (bind _returnvalue_2 (`self.Make Centimetre Vector From Metres` -0.5 (- (`KismetMathLibrary.Conv_IntToDouble` (- (`self.Height`) _index_3)) 0.5) (`KismetMathLibrary.Conv_IntToDouble` _index_3)))
        (`self.Add Instance At Location` _returnvalue_2 (struct) (`self.Triangle Left Panels`) (struct :`G` 1.0 :`A` 1.0))
        (`self.Add Instance At Location` (* _returnvalue_2 (1.0 -1.0 1.0)) (struct) (`self.Triangle Right Panels`) (struct :`G` 1.0 :`A` 1.0))))))

(fn `Generate Hanging Lights (TODO)`)

(fn `Generate Side Rafters (TODO)`)

(fn `Generate Side Walls`
  (`|ExecutionSequence`
    (:`then_0`
      ;[1 1 1] Set Meshes
      (`StaticMeshComponent.SetStaticMesh` (`self.Side Square Panels`) (`self.SideMesh`)))
    (:`then_1`
      (for _index (range (`self.Length`))
        (for _index_2 (range (`self.Height`))
          (bind _returnvalue (`KismetMathLibrary.Conv_IntToDouble` _index_2))
          (bind _returnvalue_2 (`self.Make Centimetre Vector From Metres` (`KismetMathLibrary.Conv_IntToDouble` _index) (- (`KismetMathLibrary.Conv_IntToDouble` (`self.Height`)) _returnvalue) _returnvalue))
          (`self.Add Instance At Location` _returnvalue_2 (struct :`Yaw` -90.0) (`self.Side Square Panels`) (struct :`G` 1.0 :`A` 1.0))
          (`self.Add Instance At Location` (* _returnvalue_2 (1.0 -1.0 1.0)) (struct :`Yaw` 90.0) (`self.Side Square Panels`) (struct :`G` 1.0 :`A` 1.0)))))))

(fn `Generate Support Struts (TODO)`)

(fn `UserConstructionScript`
  (`|ExecutionSequence`
    (:`then_0`
      (`KismetSystemLibrary.FlushPersistentDebugLines`))
    (:`then_1`
      (`self.Generate Floor`))
    (:`then_2`
      (`self.Generate Side Walls`))
    (:`then_3`
      (`self.Generate Side Rafters (TODO)`))
    (:`then_4`
      (`self.Generate Front Wall`))
    (:`then_5`
      (`self.Generate Front Rafters (TODO)`))
    (:`then_6`
      (`self.Generate Back Wall`))
    (:`then_7`
      (`self.Generate Back Rafters (TODO)`))
    (:`then_8`
      (`self.Generate Hanging Lights (TODO)`))
    (:`then_9`
      (`self.Generate Dust Particles`))
    (:`then_10`
      (`self.Generate Focal Assets (TODO)`))
    (:`then_11`
      (if (`self.Generate Environment Meshes`)
        (`self.Generate Environmental Assets (TODO)`)))))