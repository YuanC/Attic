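; BP_RandomMeshSpawner is an attic generator Blueprint that places one randomly chosen static mesh at a random point inside a box.
; All work runs in the Construction Script, with the box extending from the actor's location by the Bound vector along world axes.
; A new component gets a random StaticMeshes entry at that point.
; Debug drawing, flushed on each construction, shows the box and chosen point.
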(fn `UserConstructionScript`
  (locals (SpawnLocation :type "Vector Structure" :default (0.0 0.0 0.0)))
  (bind _static_meshes (`self.Static Meshes`))
  (bind _returnvalue (* (- (`self.Bound`) (`KismetMathLibrary.Vector_Zero`)) (0.5 0.5 0.5)))
  (bind _returnvalue_2 (+ (`KismetMathLibrary.TransformLocation` (`self.GetTransform`)) _returnvalue))
  (`KismetSystemLibrary.FlushPersistentDebugLines`)
  (`KismetSystemLibrary.DrawDebugBox` _returnvalue_2 _returnvalue (struct :`R` 0.401042 :`G` 0.245916 :`B` 0.06494 :`A` 1.0) (struct) 5.0 3.0)
  (bind _output_get (set `local.SpawnLocation` (`KismetMathLibrary.RandomPointInBoundingBox` _returnvalue_2 _returnvalue)))
  (`KismetSystemLibrary.DrawDebugSphere` _output_get 100.0 12 (struct :`R` 1.0 :`G` 1.0 :`B` 1.0 :`A` 1.0) 10.0 5.0)
  (bind _returnvalue_3 (`AddComponent|NODE_AddStaticMeshComponent-0`))
  (`SceneComponent.K2_SetWorldLocation` _returnvalue_3 _output_get false false)
  (`StaticMeshComponent.SetStaticMesh` _returnvalue_3 (`|GetArrayItem` _static_meshes (`KismetMathLibrary.RandomIntegerInRange` 0 (`KismetArrayLibrary.Array_LastIndex` _static_meshes)))))