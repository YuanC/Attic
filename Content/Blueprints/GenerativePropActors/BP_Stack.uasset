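; BP_Stack is a generative prop actor that picks the width, height and depth of a stack.
; Generate calls Remove, then sets each dimension either to its maximum or to a value between one and that maximum drawn from RandomStream.
; The construction script and event graph are empty, and the graphs shown place no geometry.
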(fn `Generate`
  (`|ExecutionSequence`
    (:`then_0`
      (`self.Remove`))
    (:`then_1`
      ;[1 1 1] Set dimensions
      (if (`self.Set To Max Dimensions`)
        (set `self.Width` (`self.Max Width`))
        (set `self.Height` (`self.Max Height`))
        (set `self.Depth` (`self.Max Depth`))
        (else
          (set `self.Width` (`KismetMathLibrary.RandomIntegerInRangeFromStream` 1 (`self.Max Width`) (`self.Random Stream`)))
          (set `self.Height` (`KismetMathLibrary.RandomIntegerInRangeFromStream` 1 (`self.Max Height`) (`self.Random Stream`)))
          (set `self.Depth` (`KismetMathLibrary.RandomIntegerInRangeFromStream` 1 (`self.Max Depth`) (`self.Random Stream`))))))))

(fn `UserConstructionScript`)